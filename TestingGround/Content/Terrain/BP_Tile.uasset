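; BP_Tile is one segment of an infinite terrain, filled with scattered props, rocks and AI characters on BeginPlay.
; Its barrier starts locked and red, turns passable green while the player overlaps the locking volume, and calls TileConquered on entry.
; When the player enters DestroyVolume, the tile destroys itself and asks BP_InfiniteTerrainGM to spawn the next one.
; GetAttachLocation exposes the arrow's world transform as an attach point.
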(event OnComponentBeginOverlap(LockingVolumeBox)
  (params (OverlappedComponent :type Primitive%20Component%20Object%20Reference) (OtherActor :type Actor%20Object%20Reference) (OtherComp :type Primitive%20Component%20Object%20Reference) (OtherBodyIndex :type Integer) (bFromSweep :type Boolean) (SweepResult :type Hit%20Result%20Structure%20%28by%20ref%29))
  ;[1 1 1] Unlock and locking barrier
  (Utilities|IsPlayerActor OtherActor
    (:true
      (Utilities|FlowControl|Sequence
        (:then_0
          (CallFunction|Unlock))
        (:then_1
          (Class|Tile|TileConquered))))))

(event OnComponentEndOverlap(LockingVolumeBox)
  (params (OverlappedComponent :type Primitive%20Component%20Object%20Reference) (OtherActor :type Actor%20Object%20Reference) (OtherComp :type Primitive%20Component%20Object%20Reference) (OtherBodyIndex :type Integer))
  ;[1 1 1] Unlock and locking barrier
  (Utilities|IsPlayerActor OtherActor
    (:true
      (CallFunction|Lock))))

(event OnComponentBeginOverlap(DestroyVolume)
  (params (OverlappedComponent :type Primitive%20Component%20Object%20Reference) (OtherActor :type Actor%20Object%20Reference) (OtherComp :type Primitive%20Component%20Object%20Reference) (OtherBodyIndex :type Integer) (bFromSweep :type Boolean) (SweepResult :type Hit%20Result%20Structure%20%28by%20ref%29))
  ;[1 1 1] Destroy tile when player exit volume
  (Utilities|IsPlayerActor OtherActor
    (:true
      (Actor|DestroyActor)
      (CallFunction|SpawnNextTile))))

(event EventBeginPlay
  ;[1 1 1] Set this barrier to lock if player is not in it
  (CallFunction|Lock)
  (CallFunction|GenerateEnvironment)
  (Class|Tile|PlaceAIPawns "/Game/Character/Behaviour/BP_Character.BP_Character_C" (Utilities|Struct|MakeSpawnPosition 1 5 1.5e+02 1.0 1.0)))

(fn ConstructionScript)

(fn GetAttachLocation
  (return (Transformation|GetWorldTransform (Variables|Default|GetArrow))))

(fn Unlock
  (bind _barrier (Variables|Default|GetBarrier))
  (Collision|SetCollisionEnabled _barrier "NoCollision")
  (Rendering|Material|SetMaterial _barrier 0 "/Game/Terrain/Materials/MI_Barrier_Green.MI_Barrier_Green"))

(fn Lock
  (bind _barrier (Variables|Default|GetBarrier))
  (Collision|SetCollisionEnabled _barrier "QueryAndPhysics")
  (Rendering|Material|SetMaterial _barrier 0 "/Game/Terrain/Materials/MI_Barrier_Red.MI_Barrier_Red"))

(fn SpawnNextTile
  (bind _asbp_infinite_terrain_gm (Utilities|Casting|CastToBP_InfiniteTerrainGM (Game|GetGameMode)))
  (Default|SpawnTile _asbp_infinite_terrain_gm))

(fn GenerateEnvironment
  (Class|Tile|PlaceActors "/Game/Terrain/Props/BP_Container.BP_Container_C" (Utilities|Struct|MakeSpawnPosition 1 2 5e+02 1.0 1.0))
  (Class|Tile|PlaceActors "/Game/Terrain/Props/BP_Box.BP_Box_C" (Utilities|Struct|MakeSpawnPosition 1 3 1.5e+02 1.0 1.0))
  (Class|Tile|PlaceActors "/Game/Terrain/Props/BP_Canister.BP_Canister_C" (Utilities|Struct|MakeSpawnPosition 1 5 1e+02 1.0 1.0))
  (Class|Tile|PlaceActors "/Game/Terrain/Props/BP_Sacks.BP_Sacks_C" (Utilities|Struct|MakeSpawnPosition 1 1 2e+02 1.0 1.0))
  (Class|Tile|PlaceActors "/Game/Terrain/Props/BP_Rock1.BP_Rock1_C" (Utilities|Struct|MakeSpawnPosition 1 2 3.5e+02 1.0 5.0))
  (Class|Tile|PlaceActors "/Game/Terrain/Props/BP_Rock2.BP_Rock2_C" (Utilities|Struct|MakeSpawnPosition 1 3 3e+02 1.0 5.0))
  (Class|Tile|PlaceActors "/Game/Terrain/Props/BP_Rock3.BP_Rock3_C" (Utilities|Struct|MakeSpawnPosition 1 5 2e+02 1.0 5.0)))