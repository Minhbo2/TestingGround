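; AI controller for guard NPCs that sets up the PatrolData blackboard and runs the GuardBehavior tree on BeginPlay.
; Perception updates from actors without the "Enemy" tag set the blackboard enemy key when sensed and clear it when lost.
; The same updates toggle Aiming on the controlled BP_Character to match.
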(event OnTargetPerceptionUpdated(AIPerception)
  (params (Actor :type Actor%20Object%20Reference) (Stimulus :type AI%20Stimulus%20Structure))
  ;[1 1 1] On AIPer Update, get what sense this controller was trigged or updated with and report it through string. REMEMBER to give the BP_Character instance in the scene a tag of Enemy or it won't work.
  (CallFunction|UpdateBBEnemyKey Actor Actor Stimulus))

(event EventBeginPlay
  ;[1 1 1] Set and use blackboard
  (bind _blackboardcomponent (Class|AIController|UseBlackboard "/Game/Character/AI/PatrolData.PatrolData"))
  (Variables|Default|SetBBComp _blackboardcomponent)
  (AI|RunBehaviorTree "/Game/Character/AI/GuardBehavior.GuardBehavior"))

(fn ConstructionScript)

(fn UpdateBBEnemyKey
  (params (ObjectValue :type Object%20Object%20Reference) (self2 :type Actor%20Object%20Reference) (AISense :type AI%20Stimulus%20Structure))
  (bind _enemy_key (Variables|Default|GetEnemy%20Key))
  (bind _bbcomp (Variables|Default|GetBBComp))
  (if (not (Actor|ActorHasTag self2 "Enemy"))
    (if (.bSuccessfullySensed (Utilities|Struct|BreakAIStimulus AISense))
      (AI|Components|Blackboard|SetValueasObject _bbcomp _enemy_key ObjectValue) ; Set Enemy key in BB as Object to player
      (CallFunction|SetAIAiming true)
      (else
        (AI|Components|Blackboard|ClearValue _bbcomp _enemy_key)
        (CallFunction|SetAIAiming false)))))

(fn SetAIAiming
  (params (Aim :type Boolean))
  (bind _asbp_character (Utilities|Casting|CastToBP_Character (Pawn|GetControlledPawn)))
  (Variables|/Game/Character/Behaviour/BP_Character.BP_Character_C|SetAiming _asbp_character Aim))